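; Launcher weapon Blueprint that extends a parent gun class, overriding its firing and icon functions.
; StartFire calls ShootOnce, which gates shots on time since the last shot and remaining bullets.
; A valid shot decrements ammo, spawns a Bullet actor at the Muzzle transform, plays the first-person launcher fire montage on the gun owner and records the shot time.
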(fn `GetIcon`
  (returns (Icon :type "Texture2D Object Reference"))
  (return "/Game/Assets/UI/launcher_icon.launcher_icon"))

(fn `ShootOnce`
  (`parent.ShootOnce`)
  (if (>= (- (`GameplayStatics.GetTimeSeconds`) (`self.LastShootTime`)) (`self.ShootAnimTimeLength`))
    ;[1 1 1] 判断是否有子弹
    (if (> (`self.BulletNum`) 0)
      (`|ExecutionSequence`
        (:`then_0`
          ;[1 1 1] 减少子弹数
          (`/Engine/EditorBlueprintResources/StandardMacros.DecrementInt` (`self.BulletNum`)))
        (:`then_1`
          ;[1 1 1] 创建子弹
          (`|SpawnActorFromClass` "/Game/Blueprints/Bullet.Bullet_C" (`SceneComponent.K2_GetComponentToWorld` (`self.Muzzle`)) "Undefined" "OverrideRootScale" null null))
        (:`then_2`
          ;[1 1 1] 播放动画蒙太奇  抢抖动的动画
          (`Character.PlayAnimMontage` (`self.GunOwner`) "/Game/Blueprints/FppLauncherFire_Montage.FppLauncherFire_Montage" 1.0 "None"))
        (:`then_3`
          ;[1 1 1] 设置上次射击时间
          (set `self.LastShootTime` (`GameplayStatics.GetTimeSeconds`)))))))

(fn `StartFire`
  (`parent.StartFire`)
  (`|ExecutionSequence`
    (:`then_0`
      (`self.ShootOnce`))))

(fn `UserConstructionScript`
  (`parent.UserConstructionScript`))