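; Utility Blueprint that generates random full names.
; GetRandomName picks a random entry from the family name array and another from the given name array, using each array's length for the index range.
; It returns the two joined with family name first and no separator added.
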(fn `GetRandomName`
  (returns (Name :type String))
  (locals (FamilyNameArray :type "Array of String") (GivenNameArray :type "Array of String"))
  (return (`KismetStringLibrary.Concat_StrStr` (`|GetArrayItem` (`local.FamilyNameArray`) (`KismetMathLibrary.RandomIntegerInRange` 0 (- (`KismetArrayLibrary.Array_Length` (`local.FamilyNameArray`)) 1))) (`|GetArrayItem` (`local.GivenNameArray`) (`KismetMathLibrary.RandomIntegerInRange` 0 (- (`KismetArrayLibrary.Array_Length` (`local.GivenNameArray`)) 1))))))