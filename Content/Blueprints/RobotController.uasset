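; AI controller for the robot shooter enemy that hands its decision making to a behavior tree.
; BeginPlay sets up the Robot_BB blackboard and runs Robot_BT.
; An unconnected graph branch holds hard-coded logic that starts constant shooting and repeatedly moves the pawn toward the player with AIMoveTo.
; GetRobotShooter returns the controlled pawn cast to RobotShooter and is used only by that unused branch.
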(event `self.ReceiveBeginPlay`
  (`self.UseBlackboard` "/Game/Blueprints/AI/Robot_BB.Robot_BB")
  (`self.RunBehaviorTree` "/Game/Blueprints/AI/Robot_bt.Robot_BT"))

(fn `GetRobotShooter`
  (returns (RobotShooter :type "/Game/Blueprints/RobotShooter Object Reference"))
  (bind _asrobot_shooter (cast `/Game/Blueprints/RobotShooter` (`self.K2_GetPawn`)))
  (return _asrobot_shooter))

(fn `UserConstructionScript`)