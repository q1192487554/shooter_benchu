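; Shooter is a base character Blueprint for armed combatants, providing health, a gun inventory and side-based enemy checks.
; CreateGun spawns hidden guns on the RightWeapon socket and stores them in an array that is destroyed with the owner.
; TakeDamage reduces and prints health; death stops all guns, calls OnDie and detaches the controller on a short timer.
; OnDie, GetShootLocation and GetShootDirection are placeholder stubs, apparently for subclasses.
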(event `self.ReceiveDestroyed`
  ;[1 1 1] 销毁枪支
  (for _array_element (`self.Guns`)
    (`self.K2_DestroyActor` _array_element)))

(fn `CreateGun`
  (params (GunClass :type "/Game/Blueprints/Gun Class Reference"))
  ;[1 1 1] 创建抢然后放到抢数组里
  (bind _returnvalue (`|SpawnActorFromClass` GunClass (`KismetMathLibrary.MakeTransform` (0.0 0.0 0.0)) "Undefined" "OverrideRootScale" null null))
  (`self.K2_AttachToComponent` _returnvalue (`self.Mesh`) "RightWeapon" "SnapToTarget" "SnapToTarget" "SnapToTarget" true)
  (set `/Game/Blueprints/Gun.GunOwner` self _returnvalue)
  (`KismetArrayLibrary.Array_Add` (`self.Guns`) _returnvalue)
  (`self.SetActorHiddenInGame` _returnvalue true))

(fn `Die`
  ;[1 1 1] 所有枪停止开火
  (for _array_element (`self.Guns`)
    (`/Game/Blueprints/Gun.EndFire` _array_element))
  ;[1 1 1] 死亡
  (`self.OnDie`)
  ;[1 1 1] 脱离控制器控制
  (`KismetSystemLibrary.K2_SetTimer` null "DetachFromControllerPendingDestroy" 0.1))

(fn `GetCurrentGun`
  (returns (Gun :type "/Game/Blueprints/Gun Object Reference"))
  (return (`|GetArrayItem` (`self.Guns`) (`self.CurrentIndex`))))

(fn `GetShootDirection`
  (returns (Direction :type "Vector Structure"))
  (return (0.0 0.0 0.0)))

(fn `GetShootLocation`
  (returns (Location :type "Vector Structure"))
  (return (0.0 0.0 0.0)))

(fn `IsDead`
  (returns (Dead :type Boolean))
  (return (<= (`self.Health`) 0.0)))

(fn `isEnemy`
  (params (Shooter :type "/Game/Blueprints/Shooter Object Reference"))
  (returns (isEnemy :type Boolean))
  (return (!= (`/Game/Blueprints/Shooter.Side` Shooter) (`self.Side`))))

(fn `OnDie`)

(fn `TakeDamage`
  (params (Damage :type "Float (double-precision)"))
  (if (not (`self.IsDead`))
    (bind _output_get (set `self.Health` (- (`self.Health`) Damage)))
    (`KismetSystemLibrary.PrintString` (`KismetStringLibrary.Conv_DoubleToString` _output_get))
    (if (`self.IsDead`)
      ;[1 1 1] 死亡处理
      (`self.Die`))))

(fn `UserConstructionScript`
  ;[1 1 1] 构造器 子类需要调用父类构造器
  (set `self.Health` (`self.MaxHealth`)))