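; Rifle weapon Blueprint that provides automatic hitscan fire for its owning Shooter and supplies its UI icon.
; StartFire plays the montage and attached muzzle flash, then loops ShootOnce on a timer until EndFire clears them.
; ShootOnce spends a bullet and line-traces along the owner's aim with persistent debug drawing, damaging enemy Shooters, and ends fire when empty.
; An alternative multi-target trace is left unconnected.
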(fn `EndFire`
  (`parent.EndFire`)
  (if (`self.isInFire`)
    (`|ExecutionSequence`
      (:`then_0`
        (`Character.StopAnimMontage` (`self.GunOwner`) "/Game/Blueprints/FppRifil_Montage.FppRifil_Montage")
        (`ActorComponent.K2_DestroyComponent` (`self.FireEffects`)))
      (:`then_1`
        (`KismetSystemLibrary.K2_ClearTimer` null "ShootOnce"))
      (:`then_2`
        (set `self.isInFire` false)))))

(fn `GetIcon`
  (returns (Icon :type "Texture2D Object Reference"))
  (return "/Game/Assets/UI/rifle_icon.rifle_icon"))

(fn `ShootOnce`
  (bind _location (`/Game/Blueprints/Shooter.GetShootLocation` (`self.GunOwner`)))
  (`parent.ShootOnce`)
  ;[1 1 1] 判断是否有子弹 没有子弹停火
  (if (> (`self.BulletNum`) 0)
    (`|ExecutionSequence`
      (:`then_0`
        ;[1 1 1] 子弹减少
        (`/Engine/EditorBlueprintResources/StandardMacros.DecrementInt` (`self.BulletNum`)))
      (:`then_1`
        ;[1 1 1] 发射子弹
        (bind (_outhit _returnvalue) (`KismetSystemLibrary.LineTraceSingle` _location (+ (* (`KismetMathLibrary.Normal` (`/Game/Blueprints/Shooter.GetShootDirection` (`self.GunOwner`))) 1500.0) _location) "TraceTypeQuery2" false (`|MakeArray` (`self.GunOwner`) :!type "Actor Object Reference") "Persistent"))
        (if _returnvalue
          ;[1 1 1] 转化类型
          (bind _asshooter (cast `/Game/Blueprints/Shooter` (`.HitActor` (`GameplayStatics.BreakHitResult` _outhit))))
          (if (`/Game/Blueprints/Shooter.isEnemy` _asshooter (`self.GunOwner`))
            ;[1 1 1] 调用受伤函数 每次掉20滴血
            (`/Game/Blueprints/RobotShooter.TakeDamage` _asshooter 20.0 (`self.GunOwner`))))))
    (else
      (`self.EndFire`))))

(fn `StartFire`
  (`parent.StartFire`)
  ;[1 1 1] 判断是否有子弹
  (if (> (`self.BulletNum`) 0)
    (`|ExecutionSequence`
      (:`then_0`
        ;[1 1 1] 播放动画蒙太奇  抢抖动的动画
        (`Character.PlayAnimMontage` (`self.GunOwner`) "/Game/Blueprints/FppRifil_Montage.FppRifil_Montage" 1.0 "None")
        ;[1 1 1] 开枪火焰效果
        (bind _returnvalue (`GameplayStatics.SpawnEmitterAttached` "/Game/Assets/Effects/ParticleSystems/Weapons/AssaultRifle/Muzzle/P_AssaultRifle_MF.P_AssaultRifle_MF" (`self.Muzzle`)))
        ;;[1 1 1] 把粒子存在变量中 在销毁的时候用
        (set `self.FireEffects` _returnvalue))
      (:`then_1`
        ;[1 1 1] 每一次射击
        (`self.ShootOnce`)
        ;[1 1 1] 当鼠标按住的时候将额额2秒循环执行一个函数
        (`KismetSystemLibrary.K2_SetTimer` null "ShootOnce" 0.2 true))
      (:`then_2`
        ;[1 1 1] 是否开火
        (set `self.isInFire` true)))))

(fn `UserConstructionScript`
  (`parent.UserConstructionScript`))