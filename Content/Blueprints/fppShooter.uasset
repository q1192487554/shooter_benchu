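; First-person player shooter character that handles movement, mouse look, firing and weapon switching between a rifle and a launcher.
; Switching cycles the gun array by hiding and showing actors, plays an equip montage, and uses a timestamp to block firing during it.
; Shot origin and direction overrides use camera and control rotation; death pulls the camera back and ragdolls a third-person mesh.
; Z and X set or clear a test blackboard string on the first RobotController.
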(event `self.ReceiveBeginPlay`
  ;[1 1 1] 初始化创建枪支设置当前index 并且设置不隐藏
  (`self.CreateGun` "/Game/Blueprints/Rifle.Rifle_C")
  (`self.CreateGun` "/Game/Blueprints/Launcher.Launcher_C")
  (set `self.CurrentIndex` 0)
  (`self.SetActorHiddenInGame` (`self.GetCurrentGun`) false))

(event `InputAction|Equip`
  (params (Key :type "Key Structure"))
  ;[1 1 1] Q切换枪
  (:`Pressed`
    (`self.Switch Weapon`)))

(event `InputAxis|MoveForward`
  (params (AxisValue :type "Float (single-precision)"))
  ;[1 0.2172 0] 角色 前后移动
  ;;[1 1 1] 自己创建的axis事件
  ;; W和S键位事件
  (`self.AddMovementInput` (`KismetMathLibrary.GetForwardVector` (`self.GetControlRotation`)) AxisValue))

(event `InputAxis|MoveRigth`
  (params (AxisValue :type "Float (single-precision)"))
  ;[1 0.2172 0] 角色 左右移动
  ;;[1 1 1] 自己创建的axis事件
  ;; A和D键位事件
  (`self.AddMovementInput` (`KismetMathLibrary.GetRightVector` (`self.GetControlRotation`)) AxisValue))

(event `InputAxis|Turn`
  (params (AxisValue :type "Float (single-precision)"))
  ;[1 0.2172 0] 用户鼠标Y轴和X轴
  (`self.AddControllerYawInput` AxisValue))

(event `InputAxis|LookUp`
  (params (AxisValue :type "Float (single-precision)"))
  ;[1 0.2172 0] 用户鼠标Y轴和X轴
  (`self.AddControllerPitchInput` AxisValue))

(event `InputAction|Fire`
  (params (Key :type "Key Structure"))
  ;[1 0.2172 0] 开火和关火
  (:`Pressed`
    ;;[1 1 1] 自定义函数   开火和停止开火
    (`self.StartFire`))
  (:`Released`
    (`self.EndFire`)))

(event `Key|Z`
  (params (Key :type "Key Structure"))
  (:`Pressed`
    (bind _outactors (`GameplayStatics.GetAllActorsOfClass` "/Game/Blueprints/RobotController.RobotController_C"))
    (`BlackboardComponent.SetValueAsString` (`AIBlueprintHelperLibrary.GetBlackboard` (`|GetArrayItem` _outactors)) "TestString" "Hello")))

(event `Key|X`
  (params (Key :type "Key Structure"))
  (:`Pressed`
    (bind _outactors (`GameplayStatics.GetAllActorsOfClass` "/Game/Blueprints/RobotController.RobotController_C"))
    (`BlackboardComponent.SetValueAsString` (`AIBlueprintHelperLibrary.GetBlackboard` (`|GetArrayItem` _outactors)) "TestString" "")))

(fn `EndFire`
  (`/Game/Blueprints/Gun.EndFire` (`self.GetCurrentGun`)))

(fn `GetShootDirection`
  (returns (Direction :type "Vector Structure"))
  (return (`KismetMathLibrary.GetForwardVector` (`self.GetControlRotation`))))

(fn `GetShootLocation`
  (returns (Location :type "Vector Structure"))
  ;[1 1 1] 重载 获取相机位置
  (return (`SceneComponent.K2_GetComponentLocation` (`self.Camera`))))

(fn `isInEquip`
  (returns (Equipping :type Boolean))
  (return (< (- (`GameplayStatics.GetTimeSeconds`) (`self.EquipTime`)) (`self.EquipTimeLength`))))

(fn `OnDie`
  (bind _mesh (`self.Mesh`))
  (`parent.OnDie`)
  (`SceneComponent.K2_AddLocalOffset` (`self.Camera`) (-400.0 0.0 0.0) false false)
  (`SkinnedMeshComponent.SetSkinnedAssetAndUpdate` _mesh "/Game/Assets/Characters/Models/HeroTPP.HeroTPP" true)
  (`PrimitiveComponent.SetSimulatePhysics` _mesh true)
  (`PrimitiveComponent.SetCollisionEnabled` _mesh "QueryAndPhysics"))

(fn `StartFire`
  (if (not (`self.isInEquip`))
    (`/Game/Blueprints/Gun.StartFire` (`self.GetCurrentGun`))))

(fn `Switch Weapon`
  (if (not (`self.isInEquip`))
    (`|ExecutionSequence`
      (:`then_0`
        ;[1 1 1] 切枪时候状态复位
        (`/Game/Blueprints/Gun.EndFire` (`self.GetCurrentGun`)))
      (:`then_1`
        (`self.SetActorHiddenInGame` (`self.GetCurrentGun`) true)
        (set `self.CurrentIndex` (mod (+ (`self.CurrentIndex`) 1) (`KismetArrayLibrary.Array_Length` (`self.Guns`)))))
      (:`then_2`
        (`self.SetActorHiddenInGame` (`self.GetCurrentGun`) false))
      (:`then_3`
        ;[1 1 1] 播放换枪动画
        (`self.PlayAnimMontage` "/Game/Blueprints/FppEquip_Montage.FppEquip_Montage"))
      (:`then_4`
        (set `self.EquipTime` (`GameplayStatics.GetTimeSeconds`))))))

(fn `UserConstructionScript`)